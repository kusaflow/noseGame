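; Test actor that carries the player along a spline path when the main character enters its trigger box.
; The box overlap plays a montage on that character and starts a timeline.
; Each timeline update scales the spline's length by the timeline value and snaps player pawn 0 to that world location without sweep.
; The actor destroys itself when the timeline finishes.
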(event `self.Box.OnComponentBeginOverlap`
  (params (OverlappedComponent :type "PrimitiveComponent Object Reference") (OtherActor :type "Actor Object Reference") (OtherComp :type "PrimitiveComponent Object Reference") (OtherBodyIndex :type Integer) (bFromSweep :type Boolean) (SweepResult :type "HitResult Structure (by ref)"))
  (bind _spline (`self.Spline`))
  (bind _asmain_char (cast `mainChar` OtherActor))
  (`Character.PlayAnimMontage` _asmain_char (`self.montage`) 1.0 "None")
  (bind (_direction _data) (`Timeline|Timeline_0`)
    (:`Update`
      (`self.K2_SetActorLocation` (`GameplayStatics.GetPlayerPawn` 0) (`SplineComponent.GetLocationAtDistanceAlongSpline` _spline (* _data (`SplineComponent.GetSplineLength` _spline)) "World") false false))
    (:`Finished`
      (`self.K2_DestroyActor`))))

(fn `UserConstructionScript`)