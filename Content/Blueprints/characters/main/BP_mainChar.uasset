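; BP_mainChar is the main character Blueprint, with forward-axis movement and a Q-triggered scan effect driven through the ScanPara material parameter collection.
; Tick writes the capsule's world location to the collection, and pressing Q restarts a timeline that animates its radius parameter.
; A separate event stores local forward velocity in VelForAnim, apparently for animation, while TestTick is an empty stub called every tick.
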(event `self.ReceiveTick`
  (params (DeltaSeconds :type "Float (single-precision)"))
  (`self.TestTick`)
  (`KismetMaterialLibrary.SetVectorParameterValue` "/Game/utils/postprocessing/scanEffect/scanPara.scanPara" "locOfPlayer" (`KismetMathLibrary.Conv_VectorToLinearColor` (`SceneComponent.K2_GetComponentLocation` (`self.CapsuleComponent`)))))

(event `self.SetVelForAnim`
  (bind _rootcomponent (`self.RootComponent`))
  ;[1 1 1] rotation
  (set `self.velForAnim` (.x (`KismetMathLibrary.LessLess_VectorRotator` (`SceneComponent.GetComponentVelocity` _rootcomponent) (`SceneComponent.K2_GetComponentRotation` _rootcomponent)))))

(event `Key|Q`
  (params (Key :type "Key Structure"))
  (:`Pressed`
    (bind (_direction _newtrack_0) (`Timeline|Timeline_0` :!via `PlayFromStart`)
      (:`Update`
        (`KismetMaterialLibrary.SetScalarParameterValue` "/Game/utils/postprocessing/scanEffect/scanPara.scanPara" "radius" _newtrack_0)))))

(event `InputAxis|test`
  (params (AxisValue :type "Float (single-precision)"))
  (`self.AddMovementInput` (`SceneComponent.GetForwardVector` (`self.CapsuleComponent`)) AxisValue))

(event `TestTick`)

(fn `UserConstructionScript`)